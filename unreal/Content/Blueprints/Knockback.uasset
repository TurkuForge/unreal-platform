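; Knockback actor that, on BeginPlay, launches Characters overlapping player character 0.
; Each launch adds velocity built from the unit direction from that Character toward this actor's root, multiplied componentwise by a random cone vector.
; The cone has zero half-angle along X and returns a unit vector, so the launch keeps only the X component, at most one unit in magnitude.
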(event `self.ReceiveBeginPlay`
  (for _array_element (`self.GetOverlappingActors` (`GameplayStatics.GetPlayerCharacter` 0) null)
    (bind _ascharacter (cast `Character` _array_element))
    (`Character.LaunchCharacter` _ascharacter (* (`KismetMathLibrary.GetDirectionUnitVector` (`self.K2_GetActorLocation` _ascharacter) (`SceneComponent.K2_GetComponentLocation` (`self.DefaultSceneRoot`))) (`KismetMathLibrary.RandomUnitVectorInConeInDegrees` (60.0 0.0 0.0))) false false)))

(fn `UserConstructionScript`)